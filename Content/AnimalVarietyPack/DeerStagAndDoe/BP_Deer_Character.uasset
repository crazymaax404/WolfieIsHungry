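; Deer prey character that wanders and grazes at random navigable points and flees from the player's wolf.
; Perception of the wolf or damage starts a faster run to a point ahead of the wolf, repeated depending on a sphere-trace check for the wolf.
; Damage updates a health-bar widget, shown while the player overlaps a sphere.
; At zero health it plays a death montage, stops movement, unpossesses and flags the AnimBP dead.
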(event OnPerceptionUpdated(AIPerception)
  (params (UpdatedActors :type Array%20of%20Actor%20Object%20References))
  (bind _returnvalue (Transformation|GetActorLocation))
  ;[1 1 1] AI Perception
  (for _array_element UpdatedActors
    (bind _returnvalue_2 (Actor|GetActorOfClass "/Game/AnimalVarietyPack/Wolf/BP_Wolf_Character.BP_Wolf_Character_C"))
    (if (== _returnvalue_2 _array_element)
      (bind _asabp_deer (Utilities|Casting|CastToABP_Deer (Components|SkeletalMesh|GetAnimInstance (Variables|Character|GetMesh))))
      (Variables|/Game/AnimalVarietyPack/DeerStagAndDoe/Animations/ABP_Deer.ABP_Deer_C|SetisEating _asabp_deer false)
      (bind _asbp_wolf_character (Utilities|Casting|CastToBP_Wolf_Character (Game|GetPlayerCharacter 0)))
      (Variables|Default|SetWolfBP _asbp_wolf_character)
      (if (not (Variables|Default|GetisBeingChased))
        (Variables|Default|SetisBeingChased true)
        (Variables|/Script/Engine.CharacterMovementComponent|SetMaxWalkSpeed (Variables|Character|GetCharacterMovement) 4e+02)
        (AI|AIMoveTo self (+ (Transformation|GetActorLocation (Variables|Default|GetWolfBP)) (* (Transformation|GetActorForwardVector (Variables|Default|GetWolfBP)) 2e+03)) 0 5.0 false
          (:OnSuccess
            _)
          (:OnFail
            _))
        (bind _outhits (Collision|MultiSphereTraceByChannel _returnvalue _returnvalue 5e+02 "TraceTypeQuery1" false 0 "ForDuration"))
        (bind _array_element_2 (Utilities|Array|ForEachLoopwithBreak _outhits :!label _label)
          (:LoopBody
            (bind _returnvalue_3 (Actor|GetActorOfClass "/Game/AnimalVarietyPack/Wolf/BP_Wolf_Character.BP_Wolf_Character_C"))
            (if (== _returnvalue_3 (.hitactor _array_element_2))
              (Variables|Default|SetisBeingChased true)
              (goto _label Break)
              (else
                (Variables|Default|SetisBeingChased false))))
          (:Completed
            (if (Variables|Default|GetisBeingChased)
              (CallFunction|RunAgain)
              (else
                (Variables|/Script/Engine.CharacterMovementComponent|SetMaxWalkSpeed (Variables|Character|GetCharacterMovement) (Variables|Default|GetDefault%20Max%20Walk%20Speed))
                (CallFunction|Move)))))))))

(event OnComponentBeginOverlap(Sphere)
  (params (OverlappedComponent :type Primitive%20Component%20Object%20Reference) (OtherActor :type Actor%20Object%20Reference) (OtherComp :type Primitive%20Component%20Object%20Reference) (OtherBodyIndex :type Integer) (bFromSweep :type Boolean) (SweepResult :type Hit%20Result%20Structure%20%28by%20ref%29))
  ;[1 1 1] Show/Hide HealthBar
  (if (== OtherActor (Game|GetPlayerCharacter 0))
    (Rendering|SetVisibility (Variables|Default|GetWidget) true false)))

(event OnComponentEndOverlap(Sphere)
  (params (OverlappedComponent :type Primitive%20Component%20Object%20Reference) (OtherActor :type Actor%20Object%20Reference) (OtherComp :type Primitive%20Component%20Object%20Reference) (OtherBodyIndex :type Integer))
  ;[1 1 1] Show/Hide HealthBar
  (if (== OtherActor (Game|GetPlayerCharacter 0))
    (Rendering|SetVisibility (Variables|Default|GetWidget) false false)))

(event Custom|Move
  ;[1 1 1] Random Movement
  (if (or (not (Variables|Default|GetisMoving)) (not (Variables|Default|GetisBeingChased)))
    (Variables|Default|SetisMoving true)
    (bind _randomlocation (Class|NavigationSystemV1|GetRandomLocationinNavigableRadius (Transformation|GetActorLocation) 5e+03 0 0))
    (AI|AIMoveTo self _randomlocation 0 5.0 false
      (:OnSuccess
        _)
      (:OnFail
        _))
    (Variables|Default|SetisMoving false)
    (bind _asabp_deer (Utilities|Casting|CastToABP_Deer (Components|SkeletalMesh|GetAnimInstance (Variables|Character|GetMesh))))
    (Variables|/Game/AnimalVarietyPack/DeerStagAndDoe/Animations/ABP_Deer.ABP_Deer_C|SetisEating _asabp_deer true)
    (Utilities|FlowControl|Delay 5.0)
    (Variables|/Game/AnimalVarietyPack/DeerStagAndDoe/Animations/ABP_Deer.ABP_Deer_C|SetisEating _asabp_deer false)
    (CallFunction|Move)))

(event Custom|Run%20Again
  (bind _returnvalue (Transformation|GetActorLocation))
  (bind _wolfbp (Variables|Default|GetWolfBP))
  ;[1 1 1] AI Perception
  (AI|AIMoveTo self (+ (Transformation|GetActorLocation _wolfbp) (* (Transformation|GetActorForwardVector _wolfbp) 2e+03)) 0 5.0 false
    (:OnSuccess
      _)
    (:OnFail
      _))
  (bind _outhits (Collision|MultiSphereTraceByChannel _returnvalue _returnvalue 5e+02 "TraceTypeQuery1" false 0 "ForDuration"))
  (bind _array_element (Utilities|Array|ForEachLoopwithBreak _outhits :!label _label)
    (:LoopBody
      (bind _returnvalue_2 (Actor|GetActorOfClass "/Game/AnimalVarietyPack/Wolf/BP_Wolf_Character.BP_Wolf_Character_C"))
      (if (== _returnvalue_2 (.hitactor _array_element))
        (Variables|Default|SetisBeingChased true)
        (goto _label Break)
        (else
          (Variables|Default|SetisBeingChased false))))
    (:Completed
      (if (Variables|Default|GetisBeingChased)
        (CallFunction|RunAgain)
        (else
          (Variables|/Script/Engine.CharacterMovementComponent|SetMaxWalkSpeed (Variables|Character|GetCharacterMovement) (Variables|Default|GetDefault%20Max%20Walk%20Speed))
          (CallFunction|Move))))))

(event Custom|Damage%20Received
  (bind _returnvalue (Transformation|GetActorLocation))
  ;[1 1 1] AI Perception
  (bind _asabp_deer (Utilities|Casting|CastToABP_Deer (Components|SkeletalMesh|GetAnimInstance (Variables|Character|GetMesh))))
  (Variables|/Game/AnimalVarietyPack/DeerStagAndDoe/Animations/ABP_Deer.ABP_Deer_C|SetisEating _asabp_deer false)
  (bind _asbp_wolf_character (Utilities|Casting|CastToBP_Wolf_Character (Game|GetPlayerCharacter 0)))
  (Variables|Default|SetWolfBP _asbp_wolf_character)
  (if (not (Variables|Default|GetisBeingChased))
    (Variables|Default|SetisBeingChased true)
    (Variables|/Script/Engine.CharacterMovementComponent|SetMaxWalkSpeed (Variables|Character|GetCharacterMovement) 4e+02)
    (AI|AIMoveTo self (+ (Transformation|GetActorLocation (Variables|Default|GetWolfBP)) (* (Transformation|GetActorForwardVector (Variables|Default|GetWolfBP)) 2e+03)) 0 5.0 false
      (:OnSuccess
        _)
      (:OnFail
        _))
    (bind _outhits (Collision|MultiSphereTraceByChannel _returnvalue _returnvalue 5e+02 "TraceTypeQuery1" false 0 "ForDuration"))
    (bind _array_element (Utilities|Array|ForEachLoopwithBreak _outhits :!label _label)
      (:LoopBody
        (bind _returnvalue_2 (Actor|GetActorOfClass "/Game/AnimalVarietyPack/Wolf/BP_Wolf_Character.BP_Wolf_Character_C"))
        (if (== _returnvalue_2 (.hitactor _array_element))
          (Variables|Default|SetisBeingChased true)
          (goto _label Break)
          (else
            (Variables|Default|SetisBeingChased false))))
      (:Completed
        (if (Variables|Default|GetisBeingChased)
          (CallFunction|RunAgain)
          (else
            (Variables|/Script/Engine.CharacterMovementComponent|SetMaxWalkSpeed (Variables|Character|GetCharacterMovement) (Variables|Default|GetDefault%20Max%20Walk%20Speed))
            (CallFunction|Move)))))))

(event EventBeginPlay
  ;[1 1 1] Random Movement
  (Utilities|FlowControl|Sequence
    (:then_0
      (if (or (not (Variables|Default|GetisMoving)) (not (Variables|Default|GetisBeingChased)))
        (Variables|Default|SetisMoving true)
        (bind _randomlocation (Class|NavigationSystemV1|GetRandomLocationinNavigableRadius (Transformation|GetActorLocation) 5e+03 0 0))
        (AI|AIMoveTo self _randomlocation 0 5.0 false
          (:OnSuccess
            _)
          (:OnFail
            _))
        (Variables|Default|SetisMoving false)
        (bind _asabp_deer (Utilities|Casting|CastToABP_Deer (Components|SkeletalMesh|GetAnimInstance (Variables|Character|GetMesh))))
        (Variables|/Game/AnimalVarietyPack/DeerStagAndDoe/Animations/ABP_Deer.ABP_Deer_C|SetisEating _asabp_deer true)
        (Utilities|FlowControl|Delay 5.0)
        (Variables|/Game/AnimalVarietyPack/DeerStagAndDoe/Animations/ABP_Deer.ABP_Deer_C|SetisEating _asabp_deer false)
        (CallFunction|Move)))
    (:then_1
      (Variables|Default|SetDefault%20Max%20Walk%20Speed (Variables|/Script/Engine.CharacterMovementComponent|GetMaxWalkSpeed (Variables|Character|GetCharacterMovement))))
    (:then_2
      ;;[1 1 1] Create Heath Widget
      (bind _returnvalue (UserInterface|CreateWidget "/Game/UI/WBP_Deer_HealthBar.WBP_Deer_HealthBar_C"))
      (bind _output_get (Variables|Default|SetHealthWidget _returnvalue))
      (UserInterface|SetWidget (Variables|Default|GetWidget) _output_get))))

(event Game|Damage|EventAnyDamage
  (params (Damage :type Float%20%28single-precision%29) (DamageType :type Damage%20Type%20Object%20Reference) (InstigatedBy :type Controller%20Object%20Reference) (DamageCauser :type Actor%20Object%20Reference))
  ;[1 1 1] Damage System
  (bind _output_get (Variables|Default|SetHealth (- (Variables|Default|GetHealth) Damage)))
  (CallFunction|DamageReceived)
  (Variables|/Game/UI/WBP_Deer_HealthBar.WBP_Deer_HealthBar_C|SetHealth (Variables|Default|GetHealthWidget) (/ (Variables|Default|GetHealth) 1e+02))
  (if (<= _output_get 0.0)
    (Utilities|FlowControl|DoOnce false
      (:Completed
        (Animation|PlayAnimMontage "/Game/AnimalVarietyPack/DeerStagAndDoe/Animations/ANIM_DeerStag_Death_Montage.ANIM_DeerStag_Death_Montage" 1.0 "None")
        (Pawn|Components|CharacterMovement|DisableMovement (Variables|Character|GetCharacterMovement))
        (Pawn|UnPossess (AI|GetAIController self))
        (Utilities|FlowControl|Delay 2.0)
        (bind _asabp_deer (Utilities|Casting|CastToABP_Deer (Components|SkeletalMesh|GetAnimInstance (Variables|Character|GetMesh))))
        (Variables|/Game/AnimalVarietyPack/DeerStagAndDoe/Animations/ABP_Deer.ABP_Deer_C|SetisDead _asabp_deer true)
        (Rendering|SetVisibility (Variables|Default|GetWidget) false false)))))

(fn ConstructionScript)